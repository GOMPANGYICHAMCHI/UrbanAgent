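; Main title game mode that runs the front-end flow from title screen to entry menu.
; On BeginPlay it shows the animated title widget and plays looping-agnostic title BGM, with a next-panel callback bound.
; SpawnEntry hides the title, shows the entry widget and cursor, and binds its buttons and credit events.
; Menu events quit or open game, tutorial and boss speed-run levels after a delay, while credit events stop and restart the music.
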(event `CreditStart`
  (bind _titlesound (`self.TitleSound`))
  (`/Engine/EditorBlueprintResources/StandardMacros.IsValid` _titlesound
    (:`Is Valid`
      (`AudioComponent.Stop` _titlesound))))

(event `CreditEnd`
  (bind _returnvalue (`GameplayStatics.SpawnSound2D` "/Game/WorkSpace/GameDesign/YSY/Sound/MainTitleBgm.MainTitleBgm" 1.0 1.0 0.0 null))
  (set `self.TitleSound` _returnvalue))

(event `self.ReceiveBeginPlay`
  (`self.Init`))

(event `Init`
  (bind _returnvalue (`|CreateWidget` "/Game/WorkSpace/GameDesign/YSY/UI/WB_MainTitle.WB_MainTitle_C"))
  (`Widget.SetFocus` _returnvalue)
  (bind _output_get (set `self.WB_Title` _returnvalue))
  (`UserWidget.AddToViewport` _output_get 0)
  (`/Game/WorkSpace/GameDesign/YSY/UI/WB_MainTitle.StartAnimation` _output_get)
  (add `/Game/WorkSpace/GameDesign/YSY/UI/WB_MainTitle.ToNextPanel` (`self.WB_Title`) (`|CreateDelegate` :!event `SpawnEntry`))
  (bind _returnvalue_2 (`GameplayStatics.SpawnSound2D` "/Game/WorkSpace/GameDesign/YSY/Sound/MainTitleBgm.MainTitleBgm" 1.0 1.0 0.0 null))
  (set `self.TitleSound` _returnvalue_2))

(event `OnLevelLoaded_Event`)

(event `SpawnEntry`
  (`Widget.SetVisibility` (`self.WB_Title`) "Hidden")
  (bind _returnvalue (`|CreateWidget` "/Game/WorkSpace/GameDesign/YSY/UI/WB_Entry.WB_Entry_C"))
  (bind _output_get (set `self.WB_Entry` _returnvalue))
  (`UserWidget.AddToViewport` _output_get 0)
  (`/Game/WorkSpace/GameDesign/YSY/UI/WB_Entry.StartAnimation` (`self.WB_Entry`))
  (add `/Game/WorkSpace/GameDesign/YSY/UI/WB_Entry.OnClicked_btn_Credit` (`self.WB_Entry`) (`|CreateDelegate` :!event `OnClicked_btn_Credit_이벤트`))
  (add `/Game/WorkSpace/GameDesign/YSY/UI/WB_Entry.OnClicked_btn_GameSettings` (`self.WB_Entry`) (`|CreateDelegate` :!event `OnClicked_btn_GameSettings_이벤트`))
  (add `/Game/WorkSpace/GameDesign/YSY/UI/WB_Entry.OnClicked_btn_GameEnd` (`self.WB_Entry`) (`|CreateDelegate` :!event `OnClicked_btn_GameEnd_이벤트`))
  (add `/Game/WorkSpace/GameDesign/YSY/UI/WB_Entry.OnClicked_btn_Tutorial` (`self.WB_Entry`) (`|CreateDelegate` :!event `OnClicked_btn_Tutorial_이벤트`))
  (add `/Game/WorkSpace/GameDesign/YSY/UI/WB_Entry.OnClicked_btn_GameStart` (`self.WB_Entry`) (`|CreateDelegate` :!event `OnClicked_btn_GameStart_이벤트`))
  (add `/Game/WorkSpace/GameDesign/YSY/UI/WB_Entry.CreditStart` (`self.WB_Entry`) (`|CreateDelegate` :!event `CreditStart`))
  (add `/Game/WorkSpace/GameDesign/YSY/UI/WB_Entry.CreditEnd` (`self.WB_Entry`) (`|CreateDelegate` :!event `CreditEnd`))
  (add `/Game/WorkSpace/GameDesign/YSY/UI/WB_Entry.OnClicked_btn_SpeedRun` (`self.WB_Entry`) (`|CreateDelegate` :!event `OnClicked_btn_SpeedRun`))
  (set `PlayerController.bShowMouseCursor` true (`GameplayStatics.GetPlayerController` 0)))

(event `OnClicked_btn_Credit_이벤트`)

(event `OnClicked_btn_GameSettings_이벤트`)

(event `OnClicked_btn_GameEnd_이벤트`
  (`KismetSystemLibrary.QuitGame` null "Quit"))

(event `OnClicked_btn_Tutorial_이벤트`
  (`KismetSystemLibrary.Delay` 2.0)
  (`GameplayStatics.OpenLevel` "LV_TutorialMap"))

(event `OnClicked_btn_SpeedRun`
  (`KismetSystemLibrary.Delay` 2.0)
  (`GameplayStatics.OpenLevel` "LV_BossSpeedRun"))

(event `OnClicked_btn_GameStart_이벤트`
  (`KismetSystemLibrary.Delay` 2.0)
  (`GameplayStatics.OpenLevel` "LV_New3_Gate_PHI"))

(fn `UserConstructionScript`)