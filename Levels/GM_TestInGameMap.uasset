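; Test in-game map game mode that runs the stage loop, coordinating the UI manager, stage manager and character swapping components.
; Each stage spawns enemies, plays a text event and that map's level sequence, then unlocks player control and HUD.
; Bound events show the clear screen and advance stages, opening the boss level at index 3.
; On party wipe it shows a fail screen and revives both characters on Enter; F12 returns to title.
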(event `self.ReceiveBeginPlay`
  (bind _sc_characterswaping_2 (`self.SC_CharacterSwaping_2`))
  (bind _currentplayerbase (`/Game/WorkSpace/Programing/SDH/Components/SceneComponent/SC_CharacterSwaping_2.CurrentPlayerBase` (`self.SC_CharacterSwaping_2`)))
  (add `/Game/WorkSpace/GameDesign/YSY/UI/WB_Stage_Final.NodeEnd` (`/Game/WorkSpace/Programing/SDH/Components/SceneComponent/SC_UIManager.WB_Stage` (`self.SC_UIManager`)) (`|CreateDelegate` :!event `StageNodeAnimationEnd`))
  (add `/Game/WorkSpace/Programing/SDH/Components/SceneComponent/SC_StageManager.WholeStageEnd` (`self.SC_StageManager`) (`|CreateDelegate` :!event `StageEnd`))
  (add `/Game/WorkSpace/Programing/SDH/Components/SceneComponent/SC_StageManager.PlayerAllDead` (`self.SC_StageManager`) (`|CreateDelegate` :!event `PlayerAllDead`))
  (add `/Game/WorkSpace/GameDesign/YSY/UI/WB_Clear.GoToNextStage` (`/Game/WorkSpace/Programing/SDH/Components/SceneComponent/SC_UIManager.WB_Clear` (`self.SC_UIManager`)) (`|CreateDelegate` :!event `SetNextStage`))
  (add `/Game/WorkSpace/Programing/SDH/Components/SceneComponent/SC_StageManager.PlayerEneterKeyPressed` (`self.SC_StageManager`) (`|CreateDelegate` :!event `EnteryKeyPressed`))
  (`/Game/WorkSpace/GameDesign/YSY/UI/WB_Battle_Final.StartSet` (`/Game/WorkSpace/Programing/SDH/Components/SceneComponent/SC_UIManager.WB_Ingame` (`self.SC_UIManager`)))
  (`/Game/WorkSpace/Programing/SDH/Components/SceneComponent/SC_StageManager.SpawnEnemy` (`self.SC_StageManager`))
  (`/Game/WorkSpace/Programing/SDH/Actors/Players/BP_PlayerBase_2.SetControl` _currentplayerbase "NewEnumerator5" false)
  (set `/Game/WorkSpace/Programing/SDH/Actors/Players/BP_PlayerBase_2.IsMoveable` false _currentplayerbase)
  (`Widget.SetVisibility` (`/Game/WorkSpace/Programing/SDH/Components/SceneComponent/SC_UIManager.WB_Ingame` (`self.SC_UIManager`)) "Hidden")
  (`/Game/WorkSpace/GameDesign/YSY/UI/WB_MainEvent_Final.PlayTextEvent` (`/Game/WorkSpace/GameDesign/YSY/UI/WB_Stage_Final.WB_MainEvent_Final` (`/Game/WorkSpace/Programing/SDH/Components/SceneComponent/SC_UIManager.WB_Stage` (`self.SC_UIManager`))) 0)
  (for _array_element (`/Game/WorkSpace/Programing/SDH/Components/SceneComponent/SC_StageManager.MapData` (`self.SC_StageManager`))
    (bind _outactor (`LevelSequencePlayer.CreateLevelSequencePlayer` (`.LevelSequence_23_B176BBA54AF3AAA6C82EC493A3795B12` (break `/Game/WorkSpace/Programing/SDH/EnumStruct/S_StageData` _array_element))))
    (`KismetArrayLibrary.Array_Add` (`self.SelfLevelSequence`) _outactor))
  (`GameplayStatics.PlaySound2D` "/Game/WorkSpace/Art/JWW/Termica/Termica_SFX/BackGround2_Cue.BackGround2_Cue" 1.0 1.0 0.0 null null)
  (add `/Game/WorkSpace/Programing/SDH/Actors/Players/BP_PlayerBase_2.F12` (`/Game/WorkSpace/Programing/SDH/Components/SceneComponent/SC_CharacterSwaping_2.NonCurrentPlayerBase` _sc_characterswaping_2) (delegate `BackToMain`))
  (add `/Game/WorkSpace/Programing/SDH/Actors/Players/BP_PlayerBase_2.F12` (`/Game/WorkSpace/Programing/SDH/Components/SceneComponent/SC_CharacterSwaping_2.CurrentPlayerBase` _sc_characterswaping_2) (delegate `BackToMain`)))

(event `StageNodeAnimationEnd`
  (bind _currentplayerbase (`/Game/WorkSpace/Programing/SDH/Components/SceneComponent/SC_CharacterSwaping_2.CurrentPlayerBase` (`self.SC_CharacterSwaping_2`)))
  (bind _sequenceplayer (`LevelSequenceActor.SequencePlayer` (`|GetArrayItem` (`self.SelfLevelSequence`) (`/Game/WorkSpace/Programing/SDH/Components/SceneComponent/SC_StageManager.CurrentMapDataIndex` (`self.SC_StageManager`)))))
  (if (!= (`self.CurrentStageIndex`) 3)
    (`Widget.SetVisibility` (`/Game/WorkSpace/Programing/SDH/Components/SceneComponent/SC_UIManager.WB_Stage` (`self.SC_UIManager`)) "Hidden")
    (`MovieSceneSequencePlayer.Play` _sequenceplayer)
    (`KismetSystemLibrary.Delay` (`TimeManagementBlueprintLibrary.Conv_QualifiedFrameTimeToSeconds` (`MovieSceneSequencePlayer.GetEndTime` _sequenceplayer)))
    (`/Game/WorkSpace/Programing/SDH/Actors/Players/BP_PlayerBase_2.SetControl` _currentplayerbase "NewEnumerator5" true)
    (set `/Game/WorkSpace/Programing/SDH/Actors/Players/BP_PlayerBase_2.IsMoveable` true _currentplayerbase)
    (`Widget.SetVisibility` (`/Game/WorkSpace/Programing/SDH/Components/SceneComponent/SC_UIManager.WB_Ingame` (`self.SC_UIManager`)) "Visible")
    (`/Engine/EditorBlueprintResources/StandardMacros.IncrementInt` (`self.CurrentStageIndex`))
    (else
      (`GameplayStatics.OpenLevel` "LV_BossStage_Ver_3"))))

(event `BackToMain`
  (`GameplayStatics.OpenLevel` "LV_MainTitle"))

(event `StageEnd`
  (bind _currentplayerbase (`/Game/WorkSpace/Programing/SDH/Components/SceneComponent/SC_CharacterSwaping_2.CurrentPlayerBase` (`self.SC_CharacterSwaping_2`)))
  (bind _wb_clear (`/Game/WorkSpace/Programing/SDH/Components/SceneComponent/SC_UIManager.WB_Clear` (`self.SC_UIManager`)))
  (`/Game/WorkSpace/Programing/SDH/Actors/Players/BP_PlayerBase_2.SetControl` _currentplayerbase "NewEnumerator5" false)
  (set `/Game/WorkSpace/Programing/SDH/Actors/Players/BP_PlayerBase_2.IsMoveable` false _currentplayerbase)
  (`Widget.SetVisibility` _wb_clear "Visible")
  (`/Game/WorkSpace/GameDesign/YSY/UI/WB_Clear.PlayClearAnimation` _wb_clear)
  (`KismetSystemLibrary.Delay` 1.0)
  (set `/Game/WorkSpace/GameDesign/YSY/UI/WB_Clear.IsActive` true (`/Game/WorkSpace/Programing/SDH/Components/SceneComponent/SC_UIManager.WB_Clear` (`self.SC_UIManager`)))
  (set `self.IsStageClear` true))

(event `EnteryKeyPressed`
  (bind _sc_characterswaping_2 (`self.SC_CharacterSwaping_2`))
  (bind _wb_clear (`/Game/WorkSpace/Programing/SDH/Components/SceneComponent/SC_UIManager.WB_Clear` (`self.SC_UIManager`)))
  (bind _currentplayerbase (`/Game/WorkSpace/Programing/SDH/Components/SceneComponent/SC_CharacterSwaping_2.CurrentPlayerBase` _sc_characterswaping_2))
  (bind _noncurrentplayerbase (`/Game/WorkSpace/Programing/SDH/Components/SceneComponent/SC_CharacterSwaping_2.NonCurrentPlayerBase` _sc_characterswaping_2))
  (if (`self.IsAllDead`)
    (`GameplayStatics.PlaySound2D` "/Game/WorkSpace/GameDesign/YSY/Sound/ButtonHover_Menu_Cue.ButtonHover_Menu_Cue" 1.0 1.0 0.0 null null)
    (set `self.IsAllDead` false)
    (`Widget.SetVisibility` (`/Game/WorkSpace/Programing/SDH/Components/SceneComponent/SC_UIManager.WB_StageFailed` (`self.SC_UIManager`)) "Hidden")
    (`/Game/WorkSpace/Programing/SDH/Actors/Players/BP_PlayerBase_2.ReviveSelf` _currentplayerbase)
    (`/Game/WorkSpace/Programing/SDH/Actors/Players/BP_PlayerBase_2.ReviveSelf` _noncurrentplayerbase)
    (`/Game/WorkSpace/GameDesign/YSY/UI/WB_Battle_Final.SetUIVisible` (`/Game/WorkSpace/Programing/SDH/Components/SceneComponent/SC_UIManager.WB_Ingame` (`self.SC_UIManager`)) "NewEnumerator5" true)
    (`KismetSystemLibrary.K2_ClearTimer` _noncurrentplayerbase "ReviveTimer")
    (`KismetSystemLibrary.K2_ClearTimer` _currentplayerbase "ReviveTimer")
    (elif (`/Game/WorkSpace/GameDesign/YSY/UI/WB_Clear.IsActive` (`/Game/WorkSpace/Programing/SDH/Components/SceneComponent/SC_UIManager.WB_Clear` (`self.SC_UIManager`)))
      (`/Game/WorkSpace/GameDesign/YSY/UI/WB_Clear.PlayClearAnimation` _wb_clear)
      (`/Game/WorkSpace/GameDesign/YSY/UI/WB_Clear.AlterEnterkey` _wb_clear)
      (if (`self.IsStageClear`)
        (`GameplayStatics.PlaySound2D` "/Game/WorkSpace/GameDesign/YSY/Sound/ButtonHover_Menu_Cue.ButtonHover_Menu_Cue" 1.0 1.0 0.0 null null)
        (set `self.IsStageClear` false))
      (else
        (`/Game/WorkSpace/GameDesign/YSY/UI/WB_MainEvent_Final.EnterKey` (`/Game/WorkSpace/GameDesign/YSY/UI/WB_Stage_Final.WB_MainEvent_Final` (`/Game/WorkSpace/Programing/SDH/Components/SceneComponent/SC_UIManager.WB_Stage` (`self.SC_UIManager`))))))))

(event `SetNextStage`
  (`Widget.SetVisibility` (`/Game/WorkSpace/Programing/SDH/Components/SceneComponent/SC_UIManager.WB_Clear` (`self.SC_UIManager`)) "Hidden")
  (`Widget.SetVisibility` (`/Game/WorkSpace/Programing/SDH/Components/SceneComponent/SC_UIManager.WB_Stage` (`self.SC_UIManager`)) "Visible")
  (`Widget.SetVisibility` (`/Game/WorkSpace/Programing/SDH/Components/SceneComponent/SC_UIManager.WB_Ingame` (`self.SC_UIManager`)) "Hidden")
  (if (!= (`self.CurrentStageIndex`) 3)
    (`/Game/WorkSpace/Programing/SDH/Components/SceneComponent/SC_StageManager.SpawnEnemy` (`self.SC_StageManager`)))
  (`/Game/WorkSpace/GameDesign/YSY/UI/WB_MainEvent_Final.PlayTextEvent` (`/Game/WorkSpace/GameDesign/YSY/UI/WB_Stage_Final.WB_MainEvent_Final` (`/Game/WorkSpace/Programing/SDH/Components/SceneComponent/SC_UIManager.WB_Stage` (`self.SC_UIManager`))) (`self.CurrentStageIndex`)))

(event `PlayerAllDead`
  (bind _wb_stagefailed (`/Game/WorkSpace/Programing/SDH/Components/SceneComponent/SC_UIManager.WB_StageFailed` (`self.SC_UIManager`)))
  (`Widget.SetVisibility` _wb_stagefailed "Visible")
  (`/Game/WorkSpace/GameDesign/YSY/UI/WB_StageFailed.StartAnimation` _wb_stagefailed)
  (`KismetSystemLibrary.Delay` 1.0)
  (set `/Game/WorkSpace/GameDesign/YSY/UI/WB_StageFailed.IsActive` true (`/Game/WorkSpace/Programing/SDH/Components/SceneComponent/SC_UIManager.WB_StageFailed` (`self.SC_UIManager`)))
  (set `self.IsAllDead` true))

(fn `UserConstructionScript`)