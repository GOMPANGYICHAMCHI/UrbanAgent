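; Actor component that shows pop-up damage numbers on its owner by spawning BP_DamageText actors.
; PopupText spawns text at a random Y/Z offset, passing duration, rise, size and color, then attaches it to the owner with location snapped.
; With IsAccumulatedDamage on, hits add to the still-valid current text's total and reset its timer.
; Otherwise each hit spawns a new text.
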(fn `PopupText`
  (params (Damage :type "Float (double-precision)") (TextColor :type "SlateColor Structure"))
  (bind _currenttext (`self.CurrentText`))
  (bind (_returnvalue_x _returnvalue_y _returnvalue_z) (`KismetMathLibrary.BreakVector` (`Actor.K2_GetActorLocation` (`self.GetOwner`))))
  (if (`self.IsAccumulatedDamage`)
    (`/Engine/EditorBlueprintResources/StandardMacros.IsValid` (`self.CurrentText`)
      (:`Is Valid`
        (bind _output_get (set `self.AccumulatedDamage` (+ (`self.AccumulatedDamage`) (`local.Damage`))))
        (`/Game/WorkSpace/Programing/SDH/Actors/Skill/DamagePopUpText/BP_DamageText.SetDamageText` _currenttext (`KismetMathLibrary.FTrunc` _output_get))
        (`/Game/WorkSpace/Programing/SDH/Actors/Skill/DamagePopUpText/BP_DamageText.ResetTimer` _currenttext))
      (:`Is Not Valid`
        (bind _returnvalue (`|SpawnActorFromClass` "/Game/WorkSpace/Programing/SDH/Actors/Skill/DamagePopUpText/BP_DamageText.BP_DamageText_C" (`KismetMathLibrary.MakeTransform` (`KismetMathLibrary.MakeVector` _returnvalue_x (+ _returnvalue_y (`KismetMathLibrary.RandomFloatInRange` (`self.SpawnRadius`) (* (`self.SpawnRadius`) -1.0))) (+ _returnvalue_z (`KismetMathLibrary.RandomFloatInRange` (`self.SpawnRadius`) (* (`self.SpawnRadius`) 1.5))))) "Undefined" "OverrideRootScale" null (`self.DurationTime`) (`local.Damage`) (`self.RiseAmount`) (`self.TextSize`) (`local.TextColor`) true null :!label _label))
        (`Actor.K2_AttachToActor` _returnvalue (`self.GetOwner`) "None" "SnapToTarget" "KeepRelative" "KeepRelative" true)
        (bind _output_get_2 (set `self.CurrentText` _returnvalue))
        (`/Game/WorkSpace/Programing/SDH/Actors/Skill/DamagePopUpText/BP_DamageText.StartSet` _output_get_2)
        (set `self.AccumulatedDamage` (`local.Damage`))))
    (else
      (goto _label))))