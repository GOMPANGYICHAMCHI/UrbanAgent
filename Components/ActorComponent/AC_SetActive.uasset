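; AC_SetActive is an actor component that switches its owner on or off as a whole, similar to a SetActive toggle.
; Setting it active or inactive flips the owner's visibility, tick and collision together, then stores the state in ActiveSelf.
; The toggle is exposed both as the ActorSetActive event and as SetActiveFunction with identical logic, while IsActiveFunction returns the stored state.
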(event `ActorSetActive`
  (params (IsActive :type Boolean))
  (bind _returnvalue (`self.GetOwner`))
  (`Actor.SetActorHiddenInGame` _returnvalue (not IsActive))
  (`Actor.SetActorTickEnabled` _returnvalue IsActive)
  (`Actor.SetActorEnableCollision` _returnvalue IsActive)
  (set `self.ActiveSelf` IsActive))

(fn `IsActiveFunction`
  (returns (IsActive :type Boolean))
  (return (`self.ActiveSelf`)))

(fn `SetActiveFunction`
  (params (IsActive :type Boolean))
  (bind _returnvalue (`self.GetOwner`))
  (`Actor.SetActorHiddenInGame` _returnvalue (not IsActive))
  (`Actor.SetActorTickEnabled` _returnvalue IsActive)
  (`Actor.SetActorEnableCollision` _returnvalue IsActive)
  (set `self.ActiveSelf` IsActive))