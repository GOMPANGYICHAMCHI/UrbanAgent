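; Actor component that tracks an enemy's health, death and hit-point gauge.
; Damage is scaled by OffenseLevel, dispatches death at zero and, for executable enemies, flags execution at a health threshold; healing clears it above a hardcoded 15%.
; Hits fill the gauge; reaching max returns true and starts a delay timer.
; The gauge drains on Tick once its decrease flag is set, rejecting new hit points until empty.
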(event `self.ReceiveBeginPlay`
  (set `self.CurrentHealthPoint` (`self.MaxHealthPoint`)))

(event `self.ReceiveTick`
  (params (DeltaSeconds :type "Float (single-precision)"))
  (if (`self.IsDecreaseHitPoint`)
    (bind _output_get (set `self.HitPoint` (- (`self.HitPoint`) (* 10.0 (`GameplayStatics.GetWorldDeltaSeconds`)))))
    (if (<= _output_get 0.0)
      (set `self.HitPoint` 0.0)
      (set `self.IsDecreaseHitPoint` false))))

(event `SetDecreaseHitPoint`
  (set `self.IsDecreaseHitPoint` true))

(fn `GiveDamage`
  (params (DamageAmount :type "Float (double-precision)") (IsFromPlayer :type Boolean))
  (returns (IsDead :type Boolean))
  (locals (A :type "Float (double-precision)" :default 1.0) (B :type "Float (double-precision)" :default 20.0))
  (if (!= (`self.CurrentHealthPoint`) 0.0)
    (set `self.CurrentHealthPoint` (`KismetMathLibrary.FClamp` (- (`self.CurrentHealthPoint`) (* (- 1.0 (/ (- (`self.OffenseLevel`) (`local.A`)) (`local.B`))) (`local.DamageAmount`))) 0.0 (`self.MaxHealthPoint`)))
    (if (`self.IsEnemyExcutionable`)
      (if (<= (/ (`self.CurrentHealthPoint`) (`self.MaxHealthPoint`)) (`self.ExcutableHealthPercent`))
        (bind _output_get (set `self.IsCanExcution` true))
        (`self.CanExcution` _output_get)))
    (if (== (`self.CurrentHealthPoint`) 0.0)
      (`self.Death`)
      (set `self.IsDead` true))
    (return (`self.IsDead`))))

(fn `GiveHeal`
  (params (HealAmount :type "Float (double-precision)"))
  (if (not (`self.IsDead`))
    (set `self.CurrentHealthPoint` (`KismetMathLibrary.FClamp` (+ (`self.CurrentHealthPoint`) HealAmount) 0.0 (`self.MaxHealthPoint`)))
    (if (not (<= (/ (`self.CurrentHealthPoint`) (`self.MaxHealthPoint`)) 0.15))
      (bind _output_get (set `self.IsCanExcution` false))
      (`self.CanExcution` _output_get))))

(fn `GiveHitPoint`
  (returns (IsHitPointMaxed :type Boolean))
  (if (== (`self.HitPoint`) (`self.MaxHitPoint`))
    (return true)
    (elif (`self.IsDecreaseHitPoint`)
      (return false)
      (else
        (bind _output_get (set `self.HitPoint` (`KismetMathLibrary.FClamp` (+ (`self.HitPoint`) (`self.HitPointIncreaseAmount`)) 0.0 (`self.MaxHitPoint`))))
        (if (== _output_get (`self.MaxHitPoint`))
          (`KismetSystemLibrary.K2_SetTimerDelegate` (`|CreateDelegate` :!event `SetDecreaseHitPoint`) (`self.HitPointDecreaseDelay`))
          (return true)
          (else
            (return false)))))))

(fn `RatioHealth`
  (returns (RatioHealth :type "Float (double-precision)"))
  (return (/ (`self.CurrentHealthPoint`) (`self.MaxHealthPoint`))))