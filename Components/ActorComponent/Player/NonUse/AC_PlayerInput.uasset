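; Player input component that handles Enhanced Input movement, camera look, jumping and a directional dash for its owning character.
; IsMoveable gates movement and look, while SetStart supplies the movement component, camera and two probe points.
; Grounded sprint with WASD hops, turns toward the camera-relative direction, then launches along GetSprintDir's vector, angled by a downward debug-drawn trace from the points.
; A DoOnce reset by timer provides the dash cooldown.
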(event `self.ReceiveBeginPlay`
  ;[0.3021 0.3021 0.3021] Start
  (set `self.SelfChracter` (`CharacterMovementComponent.GetCharacterOwner` (`self.CharacterMovement`))))

(event `EnhancedInput|/Game/WorkSpace/Programing/SDH/Inputs/InputAction/IA_MoveForward`
  (params (ActionValue :type "Float (double-precision)") (ElapsedSeconds :type "Float (double-precision)") (TriggeredSeconds :type "Float (double-precision)") (InputAction :type "InputAction Object Reference" :default "/Game/WorkSpace/Programing/SDH/Inputs/InputAction/IA_MoveForward.IA_MoveForward"))
  (bind (_returnvalue_roll _returnvalue_pitch _returnvalue_yaw) (`KismetMathLibrary.BreakRotator` (`Pawn.GetControlRotation` (`self.SelfChracter`))))
  ;[0.1042 0.1042 0.1042] 이동
  (:`Triggered`
    (if (`self.IsMoveable`)
      (`Pawn.AddMovementInput` (`self.SelfChracter`) (`KismetMathLibrary.GetForwardVector` (`KismetMathLibrary.MakeRotator` 0.0 0.0 _returnvalue_yaw)) ActionValue false))))

(event `EnhancedInput|/Game/WorkSpace/Programing/SDH/Inputs/InputAction/IA_TurnRight`
  (params (ActionValue :type "Float (double-precision)") (ElapsedSeconds :type "Float (double-precision)") (TriggeredSeconds :type "Float (double-precision)") (InputAction :type "InputAction Object Reference" :default "/Game/WorkSpace/Programing/SDH/Inputs/InputAction/IA_TurnRight.IA_TurnRight"))
  ;[0.1042 0.1042 0.1042] 카메라 회전
  (:`Triggered`
    (if (`self.IsMoveable`)
      (`Pawn.AddControllerYawInput` (`self.SelfChracter`) ActionValue))))

(event `EnhancedInput|/Game/WorkSpace/Programing/SDH/Inputs/InputAction/IA_MoveRight`
  (params (ActionValue :type "Float (double-precision)") (ElapsedSeconds :type "Float (double-precision)") (TriggeredSeconds :type "Float (double-precision)") (InputAction :type "InputAction Object Reference" :default "/Game/WorkSpace/Programing/SDH/Inputs/InputAction/IA_MoveRight.IA_MoveRight"))
  (bind (_returnvalue_roll _returnvalue_pitch _returnvalue_yaw) (`KismetMathLibrary.BreakRotator` (`Pawn.GetControlRotation` (`self.SelfChracter`))))
  ;[0.1042 0.1042 0.1042] 이동
  (:`Triggered`
    (if (`self.IsMoveable`)
      (`Pawn.AddMovementInput` (`self.SelfChracter`) (`KismetMathLibrary.GetRightVector` (`KismetMathLibrary.MakeRotator` _returnvalue_roll 0.0 _returnvalue_yaw)) ActionValue false))))

(event `EnhancedInput|/Game/WorkSpace/Programing/SDH/Inputs/InputAction/IA_TurnUp`
  (params (ActionValue :type "Float (double-precision)") (ElapsedSeconds :type "Float (double-precision)") (TriggeredSeconds :type "Float (double-precision)") (InputAction :type "InputAction Object Reference" :default "/Game/WorkSpace/Programing/SDH/Inputs/InputAction/IA_TurnUp.IA_TurnUp"))
  ;[0.1042 0.1042 0.1042] 카메라 회전
  (:`Triggered`
    (if (`self.IsMoveable`)
      (`Pawn.AddControllerPitchInput` (`self.SelfChracter`) (* ActionValue -1.0)))))

(event `EnhancedInput|/Game/WorkSpace/Programing/SDH/Inputs/InputAction/IA_Jump`
  (params (ActionValue :type Boolean) (ElapsedSeconds :type "Float (double-precision)") (TriggeredSeconds :type "Float (double-precision)") (InputAction :type "InputAction Object Reference" :default "/Game/WorkSpace/Programing/SDH/Inputs/InputAction/IA_Jump.IA_Jump"))
  ;[0.1042 0.1042 0.1042] 점프
  (:`Triggered`
    (`Character.Jump` (`self.SelfChracter`))))

(event `EnhancedInput|/Game/WorkSpace/Programing/SDH/Inputs/InputAction/IA_Sprint`
  (params (ActionValue :type Boolean) (ElapsedSeconds :type "Float (double-precision)") (TriggeredSeconds :type "Float (double-precision)") (InputAction :type "InputAction Object Reference" :default "/Game/WorkSpace/Programing/SDH/Inputs/InputAction/IA_Sprint.IA_Sprint"))
  (bind _returnvalue (`GameplayStatics.GetPlayerController` 0))
  (bind _returnvalue_2 (`self.GetOwner`))
  (bind _playercamera (`self.PlayerCamera`))
  (bind _currentdashdirection (`self.CurrentDashDirection`))
  (bind (_returnvalue_roll _returnvalue_pitch _returnvalue_yaw) (`KismetMathLibrary.BreakRotator` (`KismetMathLibrary.RInterpTo` (`Actor.K2_GetActorRotation` _returnvalue_2) (`KismetMathLibrary.Conv_VectorToRotator` (`self.CurrentDashVector`)) (`GameplayStatics.GetWorldDeltaSeconds`))))
  ;[0.1042 0.1042 0.1042] 대쉬
  (:`Triggered`
    (if (`NavMovementComponent.IsFalling` (`self.CharacterMovement`))
      _
      (elif (`PlayerController.IsInputKeyDown` _returnvalue "A")
        (set `self.CurrentDashDirection` "A")
        (`/Engine/EditorBlueprintResources/StandardMacros.DoOnce` false :!label _label
          (:`Completed`
            (`Character.LaunchCharacter` (`self.SelfChracter`) (0.0 0.0 50.0) false false)
            (`KismetSystemLibrary.Delay` 0.01)
            (if (== _currentdashdirection "A")
              (set `self.CurrentDashVector` (* (`KismetMathLibrary.GetRightVector` (`SceneComponent.K2_GetComponentRotation` _playercamera)) -1))
              (`Actor.K2_SetActorRotation` _returnvalue_2 (`KismetMathLibrary.MakeRotator` 0.0 0.0 _returnvalue_yaw) false :!label _label_2)
              (bind _launchvelocity (`self.GetSprintDir`))
              (`Character.LaunchCharacter` (`self.SelfChracter`) (* _launchvelocity 30.0) false false)
              (if (not false)
                (`KismetSystemLibrary.K2_SetTimerDelegate` (delegate `ReDashAble`) 0.5))
              (elif (== _currentdashdirection "S")
                (set `self.CurrentDashVector` (* (`KismetMathLibrary.GetForwardVector` (`SceneComponent.K2_GetComponentRotation` _playercamera)) -1))
                (goto _label_2)
                (elif (== _currentdashdirection "D")
                  (set `self.CurrentDashVector` (`KismetMathLibrary.GetRightVector` (`SceneComponent.K2_GetComponentRotation` _playercamera)))
                  (goto _label_2)
                  (elif (== _currentdashdirection "W")
                    (set `self.CurrentDashVector` (`KismetMathLibrary.GetForwardVector` (`SceneComponent.K2_GetComponentRotation` _playercamera)))
                    (goto _label_2)))))))
        (elif (`PlayerController.IsInputKeyDown` _returnvalue "W")
          (set `self.CurrentDashDirection` "W")
          (goto _label)
          (elif (`PlayerController.IsInputKeyDown` _returnvalue "S")
            (set `self.CurrentDashDirection` "S")
            (goto _label)
            (elif (`PlayerController.IsInputKeyDown` _returnvalue "D")
              (set `self.CurrentDashDirection` "D")
              (goto _label))))))))

(event `ReDashAble`
  ;[0.1042 0.1042 0.1042] 대쉬
  (goto _label :!via `Reset`))

(fn `GetSprintDir`
  (returns (LaunchVelocity :type "Vector Structure"))
  (bind _returnvalue (`SceneComponent.K2_GetComponentLocation` (`self.Point2`)))
  (bind _returnvalue_2 (`SceneComponent.K2_GetComponentLocation` (`self.Point2`)))
  (bind _returnvalue_3 (`SceneComponent.K2_GetComponentLocation` (`self.Point1`)))
  (bind _returnvalue_4 (- _returnvalue_2 _returnvalue_3))
  (bind (_outhit _returnvalue_5) (`KismetSystemLibrary.LineTraceSingle` :`Start` _returnvalue :`End` (- _returnvalue (0.0 0.0 1000.0)) :`TraceChannel` "TraceTypeQuery3" :`DrawDebugType` "ForDuration" :`DrawTime` 2.0))
  (if _returnvalue_5
    (return (`KismetMathLibrary.RotateAngleAxis` _returnvalue_4 (`KismetMathLibrary.DegAtan` (/ (`.Distance` (`GameplayStatics.BreakHitResult` _outhit)) (`KismetMathLibrary.Vector_Distance` _returnvalue_3 _returnvalue_2))) (`KismetMathLibrary.Cross_VectorVector` _returnvalue_4 (0.0 0.0 -1.0))))
    (else
      (return (0.0 0.0 0.0)))))

(fn `SetStart`
  (params (Point1 :type "SceneComponent Object Reference") (Point2 :type "SceneComponent Object Reference") (PlayerCamera :type "CameraComponent Object Reference") (SelfCharacterMovement :type "CharacterMovementComponent Object Reference"))
  (set `self.Point1` Point1)
  (set `self.Point2` Point2)
  (set `self.PlayerCamera` PlayerCamera)
  (set `self.CharacterMovement` SelfCharacterMovement))