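; Player stat component that holds health, combat stats, shield, cooldowns and hit-point charges for skill and ultimate.
; GiveDamage applies a defense-based formula and fires PlayerDead at zero health, while EnemyHit builds the charges that gate both skills.
; Timers re-enable skills, dodge, perfect avoid and character switch, while Tick tracks elapsed time for ratio and time-left getters.
; Item-effect events adjust stats after a delay, but their callback bindings are never executed.
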(event `S001` :!signature `self.ItemEffectCallbackS001`
  (params (Delta :type "Float (double-precision)") (Duration :type "Float (double-precision)"))
  (`KismetSystemLibrary.K2_SetTimerDelegate` (delegate `S001_Timer`) Duration))

(event `W001` :!signature `self.ItemEffectCallbackW001`
  (params (Delta :type "Float (double-precision)") (Duration :type "Float (double-precision)"))
  (`KismetSystemLibrary.K2_SetTimerDelegate` (delegate `W001_Timer`) Duration))

(event `W002` :!signature `self.ItemEffectCallbackW002`
  (params (Delta :type "Float (double-precision)") (Duration :type "Float (double-precision)"))
  (`KismetSystemLibrary.K2_SetTimerDelegate` (delegate `W002_Timer`) Duration))

(event `W003` :!signature `self.ItemEffectCallbackW003`
  (params (Delta :type "Float (double-precision)") (Duration :type "Float (double-precision)"))
  (`KismetSystemLibrary.K2_SetTimerDelegate` (delegate `W003_Timer`) Duration))

(event `W004` :!signature `self.ItemEffectCallbackW004`
  (params (Delta :type "Float (double-precision)") (Duration :type "Float (double-precision)"))
  (`KismetSystemLibrary.K2_SetTimerDelegate` (delegate `W004_Timer`) Duration))

(event `E002` :!signature `self.ItemEffectCallbackE002`
  (params (Delta :type "Float (double-precision)") (Duration :type "Float (double-precision)"))
  (`KismetSystemLibrary.K2_SetTimerDelegate` (delegate `E002_Timer`) Duration))

(event `E001` :!signature `self.ItemEffectCallbackE001`
  (params (Duration :type "Float (double-precision)") (Delta :type "Float (double-precision)"))
  (`KismetSystemLibrary.K2_SetTimerDelegate` (delegate `E001_Timer`) Duration))

(event `S001_Timer`
  (set `self.DefensePower` (+ (`self.DefensePower`) (stale `S001` Delta))))

(event `W001_Timer`
  (set `self.CriticalPercent` (+ (`self.CriticalPercent`) (stale `W001` Delta))))

(event `W002_Timer`
  (set `self.CriticalDamage` (+ (`self.CriticalDamage`) (stale `W002` Delta))))

(event `E001_Timer`
  (bind _returnvalue (+ (`self.Sheild`) (stale `E001` Delta)))
  (if (> _returnvalue 0.0)
    (set `self.Sheild` _returnvalue)
    (else
      (set `self.Sheild` 0.0))))

(event `W003_Timer`
  (set `self.AttackSpeed` (+ (`self.AttackSpeed`) (stale `W003` Delta))))

(event `E002_Timer`
  (bind _returnvalue (+ (`self.Sheild`) (stale `E002` Delta)))
  (if (> _returnvalue 0.0)
    (set `self.Sheild` _returnvalue)
    (else
      (set `self.Sheild` 0.0))))

(event `W004_Timer`
  (set `self.OffensePower` (+ (`self.OffensePower`) (stale `W004` Delta))))

(event `self.ReceiveBeginPlay`
  ;[0.003922 0.003922 0.003922] 시작시 시간체크 초기화
  (set `self.TimeCheck Skill` (`self.Skill CoolTime`))
  (set `self.TimeCheck Ultimate Skill` (`self.Ultimate Skill CoolTime`))
  (set `self.TimeCheck Rotation Skill` (`self.Rotation Skill CoolTime`))
  (set `self.TimeCheck PerfectAvoid` (`self.PerfectAvoid CoolTime`))
  (set `self.TimeCheck Dash` (`self.Dash CoolTime`))
  (set `self.CurrentHealthPoint` (`self.MaxHealthPoint`)))

(event `PerfectAvoid`
  ;[0.8021 0.8021 0.8021] 완벽회피 쿨타임
  (set `self.PerfectAvoid Available` false)
  (set `self.TimeCheck PerfectAvoid` 0.0)
  (`KismetSystemLibrary.K2_SetTimerDelegate` (delegate `PerfectAvoidReset`) (`self.PerfectAvoid CoolTime`)))

(event `UseSkill`
  ;[0.08854 0.08854 0.08854] 스킬 쿨타임
  (set `self.HitPoint_Skill` (- (`self.HitPoint_Skill`) (`self.HitPointUseAmountPerSkill`)))
  (set `self.Skill Available` false)
  (set `self.TimeCheck Skill` 0.0)
  (`KismetSystemLibrary.K2_SetTimerDelegate` (delegate `ChangeSkillState`) (`self.Skill CoolTime`)))

(event `PerfectAvoidReset`
  ;[0.8021 0.8021 0.8021] 완벽회피 쿨타임
  (set `self.PerfectAvoid Available` true))

(event `ChangeSkillState`
  ;[0.08854 0.08854 0.08854] 스킬 쿨타임
  (set `self.Skill Available` true))

(event `UseUltimateSkill`
  ;[0.08854 0.08854 0.08854] 궁극기 스킬 쿨타임
  (set `self.HitPoint_UltimateSkill` 0)
  (set `self.Ultimate Skill Available` false)
  (set `self.TimeCheck Ultimate Skill` 0.0)
  (`KismetSystemLibrary.K2_SetTimerDelegate` (delegate `ChangeUltimateSkillState`) (`self.Ultimate Skill CoolTime`)))

(event `EmergencyAvoid`
  ;[0.8021 0.8021 0.8021] 긴급회피 쿨타임
  (`/Game/WorkSpace/Programing/SDH/Components/InterfaceInclude/Actor/I_EmergencyAvoid.EmergencyAvoid` (cast `/Game/WorkSpace/Programing/SDH/Components/InterfaceInclude/Actor/I_EmergencyAvoid` (`GameplayStatics.GetGameState`) :!pure true))
  (`self.EmergencyAvoidDispatch`))

(event `self.ReceiveTick`
  (params (DeltaSeconds :type "Float (single-precision)"))
  ;[0.003922 0.003922 0.003922] 업데이트 함수
  (`|ExecutionSequence`
    (:`then_0`
      (if (not (`self.Skill Available`))
        (set `self.TimeCheck Skill` (`KismetMathLibrary.FClamp` (+ (`self.TimeCheck Skill`) (`GameplayStatics.GetWorldDeltaSeconds`)) 0.0 (`self.Skill CoolTime`)))))
    (:`then_1`
      (if (not (`self.Ultimate Skill Available`))
        (set `self.TimeCheck Ultimate Skill` (`KismetMathLibrary.FClamp` (+ (`self.TimeCheck Ultimate Skill`) (`GameplayStatics.GetWorldDeltaSeconds`)) 0.0 (`self.Ultimate Skill CoolTime`)))))
    (:`then_2`
      (if (not (`self.Rotation Skill Available`))
        (set `self.TimeCheck Rotation Skill` (`KismetMathLibrary.FClamp` (+ (`self.TimeCheck Rotation Skill`) (`GameplayStatics.GetWorldDeltaSeconds`)) 0.0 (`self.Rotation Skill CoolTime`)))))
    (:`then_3`
      (if (not (`self.PerfectAvoid Available`))
        (set `self.TimeCheck PerfectAvoid` (`KismetMathLibrary.FClamp` (+ (`self.TimeCheck PerfectAvoid`) (`GameplayStatics.GetWorldDeltaSeconds`)) 0.0 (`self.PerfectAvoid CoolTime`)))))
    (:`then_4`
      (if (not (`self.Dash Available`))
        (set `self.TimeCheck Dash` (`KismetMathLibrary.FClamp` (+ (`self.TimeCheck Dash`) (`GameplayStatics.GetWorldDeltaSeconds`)) 0.0 (`self.Dash CoolTime`)))))))

(event `ChangeUltimateSkillState`
  ;[0.08854 0.08854 0.08854] 궁극기 스킬 쿨타임
  (set `self.Ultimate Skill Available` true))

(event `Dodge`
  ;[0.8021 0.8021 0.8021] 회피 쿨타임
  (set `self.Dash Available` false)
  (set `self.TimeCheck Dash` 0.0)
  (`KismetSystemLibrary.K2_SetTimerDelegate` (delegate `DodgeReset`) (`self.Dash CoolTime`)))

(event `CharacterChange`
  ;[0.08854 0.08854 0.08854] 교대기 스킬 쿨타임
  (set `self.Rotation Skill Available` false)
  (set `self.TimeCheck Rotation Skill` 0.0)
  (`KismetSystemLibrary.K2_SetTimerDelegate` (delegate `ResetCharacterChangeSkillState`) (`self.Rotation Skill CoolTime`)))

(event `DodgeReset`
  ;[0.8021 0.8021 0.8021] 회피 쿨타임
  (set `self.Dash Available` true))

(event `ResetCharacterChangeSkillState`
  ;[0.08854 0.08854 0.08854] 교대기 스킬 쿨타임
  (set `self.Rotation Skill Available` true))

(fn `EnemyHit`
  (set `self.HitPoint_Skill` (`KismetMathLibrary.Clamp` (+ (`self.HitPoint_Skill`) (`self.HitPointIncreaseAmount`)) 0 (`self.MaxHitPoint_Skill`)))
  (set `self.HitPoint_UltimateSkill` (`KismetMathLibrary.Clamp` (+ (`self.HitPoint_UltimateSkill`) (`self.HitPointIncreaseAmount`)) 0 (`self.MaxHitPoint_UltimateSkill`))))

(fn `GetDashLeftTime`
  (returns (ReturnValue :type "Float (double-precision)"))
  (return (- (`self.Dash CoolTime`) (`self.TimeCheck Dash`))))

(fn `GetPerfectAvoidLeftTime`
  (returns (ReturnValue :type "Float (double-precision)"))
  (return (- (`self.PerfectAvoid CoolTime`) (`self.TimeCheck PerfectAvoid`))))

(fn `GetRatioDash`
  (returns (ReturnRatio :type "Float (double-precision)"))
  (return (/ (`self.TimeCheck Dash`) (`self.Dash CoolTime`))))

(fn `GetRatioHealth`
  (returns (RatioHealth :type "Float (double-precision)"))
  (return (/ (`self.CurrentHealthPoint`) (`self.MaxHealthPoint`))))

(fn `GetRatioHitPoint_Skill`
  (returns (Ratio :type "Float (double-precision)") (IsHitPointUseable :type Boolean))
  (return (/ (`KismetMathLibrary.Conv_IntToDouble` (`self.HitPoint_Skill`)) (`KismetMathLibrary.Conv_IntToDouble` (`self.MaxHitPoint_Skill`))) (>= (`self.HitPoint_Skill`) (`self.HitPointUseAmountPerSkill`))))

(fn `GetRatioHitPoint_UltimateSkill`
  (returns (Ratio :type "Float (double-precision)"))
  (return (/ (`KismetMathLibrary.Conv_IntToDouble` (`self.HitPoint_UltimateSkill`)) (`KismetMathLibrary.Conv_IntToDouble` (`self.MaxHitPoint_UltimateSkill`)))))

(fn `GetRatioPerfectAvoid`
  (returns (ReturnRatio :type "Float (double-precision)"))
  (return (/ (`self.TimeCheck PerfectAvoid`) (`self.PerfectAvoid CoolTime`))))

(fn `GetRatioRotationSkill`
  (returns (ReturnRatio :type "Float (double-precision)"))
  (return (/ (`self.TimeCheck Rotation Skill`) (`self.Rotation Skill CoolTime`))))

(fn `GetRatioSkill`
  (returns (ReturnRatio :type "Float (double-precision)"))
  (return (/ (`self.TimeCheck Skill`) (`self.Skill CoolTime`))))

(fn `GetRatioUltimateSkill`
  (returns (ReturnRatio :type "Float (double-precision)"))
  (return (/ (`self.TimeCheck Ultimate Skill`) (`self.Ultimate Skill CoolTime`))))

(fn `GetRotationSkillLeftTime`
  (returns (ReturnValue :type "Float (double-precision)"))
  (return (- (`self.Rotation Skill CoolTime`) (`self.TimeCheck Rotation Skill`))))

(fn `GetSkillLeftTime`
  (returns (ReturnValue :type "Float (double-precision)"))
  (return (- (`self.Skill CoolTime`) (`self.TimeCheck Skill`))))

(fn `GetUltimateSkillLeftTime`
  (returns (ReturnValue :type "Float (double-precision)"))
  (return (- (`self.Ultimate Skill CoolTime`) (`self.TimeCheck Ultimate Skill`))))

(fn `GiveDamage`
  (params (DamageAmount :type "Float (double-precision)") (OtherOffenseLevel :type Integer))
  (locals (K :type "Float (double-precision)" :default 500.0) (N :type "Float (double-precision)" :default 100.0))
  (bind _output_get (set `self.CurrentHealthPoint` (`KismetMathLibrary.FClamp` (- (`self.CurrentHealthPoint`) (- DamageAmount (/ (`self.DefensePower`) (+ (+ (* (`local.OtherOffenseLevel`) (`local.K`)) (`local.N`)) (`self.DefensePower`))))) 0.0 (`self.MaxHealthPoint`))))
  (if (== _output_get 0.0)
    (set `self.IsDead` true)
    (`self.PlayerDead`)))

(fn `GiveHeal`
  (params (HealAmount :type "Float (double-precision)"))
  (set `self.CurrentHealthPoint` (`KismetMathLibrary.FClamp` (+ (`self.CurrentHealthPoint`) HealAmount) 0.0 (`self.MaxHealthPoint`))))

(fn `IsSkillUseable`
  (returns (Useable :type Boolean))
  (return (and (`self.Skill Available`) (>= (`self.HitPoint_Skill`) (`self.HitPointUseAmountPerSkill`)))))

(fn `IsUltimateSkillUseable`
  (returns (Useable :type Boolean))
  (return (and (`self.Ultimate Skill Available`) (== (`self.HitPoint_UltimateSkill`) (`self.MaxHitPoint_UltimateSkill`)))))