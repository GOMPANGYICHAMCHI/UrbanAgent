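; Black hole skill component that drags characters within a radius toward its owner.
; TriggerDrag captures overlapping actors once, AddTarget supplies extras, and Tick relaunches both lists inward, dropping dead or out-of-range ones.
; Optional timed damage scales with player offense, throttled by a DoOnce and timer; its flag clears permanently after the duration.
; DragDownAllPawns and Explosion apply one-off launches to captured targets, downward or along the owner axis.
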(event `OffDrag`
  (bind _array (`|MakeArray` null :!type "Actor Object Reference"))
  (set `self.IsActivate` false)
  (set `self.Targets` _array)
  (set `self.ExtraTargets` _array))

(event `TriggerDrag`
  (bind _array (`|MakeArray` null :!type "Actor Object Reference"))
  (set `self.IsActivate` true)
  (set `self.Targets` _array)
  (set `self.ExtraTargets` _array)
  (`self.SetTarget`)
  (if (`self.IsTickDamage`)
    (`KismetSystemLibrary.K2_SetTimerDelegate` (delegate `FinishTickDamaging`) (`self.TickDamageDuration`))))

(event `FinishTickDamaging`
  (set `self.IsTickDamage` false))

(event `self.ReceiveTick`
  (params (DeltaSeconds :type "Float (single-precision)"))
  (if (`self.IsActivate`)
    (`self.TargetsUpdate`)
    (`self.ExtraTargetsUpdate`)
    (if (`self.IsTickDamage`)
      (`/Engine/EditorBlueprintResources/StandardMacros.DoOnce` false :!label _label
        (:`Completed`
          (`self.GiveTickDamage`)
          (`KismetSystemLibrary.K2_SetTimerDelegate` (delegate `ResetTick`) (`self.TickTime`)))))))

(event `TickReseted`
  (goto _label :!via `Reset`))

(event `ResetTick`
  (`self.TickReseted`))

(fn `AddTarget`
  (params (AddTarget :type "Actor Object Reference"))
  (`KismetArrayLibrary.Array_Add` (`self.ExtraTargets`) AddTarget))

(fn `DragDownAllPawns`
  (for _array_element (`self.Targets`)
    (`Character.LaunchCharacter` (cast `Character` _array_element :!pure true) (* (`Actor.GetActorUpVector` _array_element) -1000.0) false false)))

(fn `DraggingEnemy(DUMP)`
  (bind _blackholeradius (`self.BlackHoleRadius`))
  (bind _returnvalue (`Actor.K2_GetActorLocation` (`self.GetOwner`)))
  (`|ExecutionSequence`
    (:`then_0`
      (`KismetSystemLibrary.DrawDebugSphere` _returnvalue _blackholeradius 16 (struct :`G` 1.0 :`B` 0.880471 :`A` 1.0) 5.0 1.0))
    (:`then_1`
      (bind _outactors (`KismetSystemLibrary.SphereOverlapActors` _returnvalue _blackholeradius (`self.ObjectType`) "/Script/Engine.Actor"))
      (for _array_element _outactors
        (bind _ascharacter (cast `Character` _array_element :!pure true))
        (`/Engine/EditorBlueprintResources/StandardMacros.IsValid` _ascharacter
          (:`Is Valid`
            (`Character.LaunchCharacter` _ascharacter (+ (* (`KismetMathLibrary.Normal` (- (`Actor.K2_GetActorLocation` (`self.GetOwner`)) (`Actor.K2_GetActorLocation` _array_element))) (`self.DragAmount`)) (0.0 0.0 100.0)) false false)))))))

(fn `Explosion`
  (for _array_element (`self.Targets`)
    (`Character.LaunchCharacter` (cast `Character` _array_element :!pure true) (* (`KismetMathLibrary.Normal` (- (`Actor.K2_GetActorLocation` (`self.GetOwner`)) (`Actor.K2_GetActorLocation` _array_element))) (`self.ExplosionAmount`)) false false)))

(fn `ExtraTargetsUpdate`
  (for _array_element (`self.ExtraTargets`)
    (if (`self.IsActivate`)
      (`/Engine/EditorBlueprintResources/StandardMacros.IsValid` _array_element
        (:`Is Valid`
          (if (`/Game/WorkSpace/Programing/SDH/Components/ActorComponent/Enemy/AC_EnemyStat.IsDead` (`Actor.GetComponentByClass` _array_element "/Game/WorkSpace/Programing/SDH/Components/ActorComponent/Enemy/AC_EnemyStat.AC_EnemyStat_C"))
            (`KismetArrayLibrary.Array_RemoveItem` (`self.ExtraTargets`) _array_element :!label _label)
            (elif (> (`KismetMathLibrary.Vector_Distance` (`Actor.K2_GetActorLocation` (`self.GetOwner`)) (`Actor.K2_GetActorLocation` _array_element)) (`self.BlackHoleRadius`))
              (goto _label)
              (elif (<= (`KismetMathLibrary.Vector_Distance` (`Actor.K2_GetActorLocation` (`self.GetOwner`)) (`Actor.K2_GetActorLocation` _array_element)) (`self.MinDistance`))
                (bind _ascharacter (cast `Character` _array_element :!pure true))
                (`Character.LaunchCharacter` _ascharacter (`self.AdjustAmount`) false false)
                (else
                  (`Character.LaunchCharacter` _ascharacter (+ (* (`KismetMathLibrary.Normal` (- (`Actor.K2_GetActorLocation` (`self.GetOwner`)) (`Actor.K2_GetActorLocation` _array_element))) (`self.DragAmount`)) (`self.AdjustAmount`)) false false))))))
        (:`Is Not Valid`
          (goto _label)))
      (else
        (break)))))

(fn `GiveTickDamage`
  (locals (ActorLocation :type "Vector Structure"))
  ;[1 1 1] 초기설정
  (set `local.ActorLocation` (`Actor.K2_GetActorLocation` (`self.GetOwner`)))
  (for _array_element (`self.Targets`)
    (bind _asi_damage_able (cast `/Game/WorkSpace/Programing/SDH/Components/InterfaceInclude/Actor/I_DamageAble` _array_element))
    (`/Game/WorkSpace/Programing/SDH/Components/InterfaceInclude/Actor/I_DamageAble.GiveDamage` _asi_damage_able (* (`self.TickDamagePercent`) (`/Game/WorkSpace/Programing/SDH/Components/ActorComponent/Player/Base/AC_PlayerStat.OffensePower` (`self.PlayerStat`))) 0 (`local.ActorLocation`) false false))
  (for _array_element_2 (`self.ExtraTargets`)
    (bind _asi_damage_able_2 (cast `/Game/WorkSpace/Programing/SDH/Components/InterfaceInclude/Actor/I_DamageAble` _array_element_2))
    (`/Game/WorkSpace/Programing/SDH/Components/InterfaceInclude/Actor/I_DamageAble.GiveDamage` _asi_damage_able_2 (* (`self.TickDamagePercent`) (`/Game/WorkSpace/Programing/SDH/Components/ActorComponent/Player/Base/AC_PlayerStat.OffensePower` (`self.PlayerStat`))) 0 (`local.ActorLocation`) false false)))

(fn `SetTarget`
  (bind _blackholeradius (`self.BlackHoleRadius`))
  (bind _returnvalue (`Actor.K2_GetActorLocation` (`self.GetOwner`)))
  (`|ExecutionSequence`
    (:`then_0`
      (`KismetSystemLibrary.DrawDebugSphere` _returnvalue _blackholeradius 16 (struct :`G` 1.0 :`B` 0.880471 :`A` 1.0) 5.0 1.0))
    (:`then_1`
      (bind _outactors (`KismetSystemLibrary.SphereOverlapActors` _returnvalue _blackholeradius (`self.ObjectType`) "/Script/Engine.Actor"))
      (set `self.Targets` _outactors))))

(fn `TargetsUpdate`
  (for _array_element (`self.Targets`)
    (if (`self.IsActivate`)
      (if (`/Game/WorkSpace/Programing/SDH/Components/ActorComponent/Enemy/AC_EnemyStat.IsDead` (`Actor.GetComponentByClass` _array_element "/Game/WorkSpace/Programing/SDH/Components/ActorComponent/Enemy/AC_EnemyStat.AC_EnemyStat_C"))
        (`KismetArrayLibrary.Array_RemoveItem` (`self.Targets`) _array_element :!label _label)
        (elif (> (`KismetMathLibrary.Vector_Distance` (`Actor.K2_GetActorLocation` (`self.GetOwner`)) (`Actor.K2_GetActorLocation` _array_element)) (`self.BlackHoleRadius`))
          (goto _label)
          (elif (<= (`KismetMathLibrary.Vector_Distance` (`Actor.K2_GetActorLocation` (`self.GetOwner`)) (`Actor.K2_GetActorLocation` _array_element)) (`self.MinDistance`))
            (bind _ascharacter (cast `Character` _array_element :!pure true))
            (`Character.LaunchCharacter` _ascharacter (`self.AdjustAmount`) false false)
            (else
              (`Character.LaunchCharacter` _ascharacter (+ (* (`KismetMathLibrary.Normal` (- (`Actor.K2_GetActorLocation` (`self.GetOwner`)) (`Actor.K2_GetActorLocation` _array_element))) (`self.DragAmount`)) (`self.AdjustAmount`)) false false)))))
      (else
        (break)))))