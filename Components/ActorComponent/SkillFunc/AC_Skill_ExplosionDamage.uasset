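; Skill actor component that applies radial explosion damage or healing around its owner, or only returns the affected actors.
; BeginPlay picks target object types from ForAll and IsFromPlayer.
; CalculateExplosionDamage sphere-overlaps those types, then line-traces to each actor's bounds center and offset points, so cover can block the blast.
; The first trace hitting the actor counts; PenetrateTarget makes traces ignore other overlapped actors.
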(event `self.ReceiveBeginPlay`
  (if (`self.ForAll`)
    (set `self.ExplosionTarget` (`|MakeArray` "ObjectTypeQuery7" "ObjectTypeQuery8" :!type "EObjectTypeQuery Enum"))
    (elif (`self.IsFromPlayer`)
      (set `self.ExplosionTarget` (`|MakeArray` "ObjectTypeQuery7" :!type "EObjectTypeQuery Enum"))
      (else
        (set `self.ExplosionTarget` (`|MakeArray` "ObjectTypeQuery8" :!type "EObjectTypeQuery Enum"))))))

(fn `CalculateExplosionDamage`
  (params (DebugCircle :type Boolean))
  (returns (HitTargets :type "Array of Actor Object Reference"))
  (locals (IgnoreList :type "Array of Actor Object Reference") (ReturnActor :type "Array of Actor Object Reference"))
  (bind _explosionradius (`self.ExplosionRadius`))
  (bind _returnvalue (`Actor.K2_GetActorLocation` (`self.GetOwner`)))
  (`|ExecutionSequence`
    (:`then_0`
      (if DebugCircle
        (`KismetSystemLibrary.DrawDebugSphere` _returnvalue _explosionradius 16 (struct :`G` 1.0 :`B` 0.880471 :`A` 1.0) 5.0 1.0)))
    (:`then_1`
      (bind _outactors (`KismetSystemLibrary.SphereOverlapActors` _returnvalue _explosionradius (`self.ExplosionTarget`) "/Script/Engine.Actor"))
      (for _array_element _outactors
        (if (`self.PenetrateTarget`)
          (bind _output_get (set `local.IgnoreList` _outactors))
          (`KismetArrayLibrary.Array_RemoveItem` _output_get _array_element))
        (if (`KismetSystemLibrary.IsValid` _array_element)
          (bind (_origin _boxextent) (`Actor.GetActorBounds` _array_element true true))
          (bind _corners (`self.GetBoxCorners` _origin _boxextent))
          (for _array_element_2 _corners
            (bind _outhit (`KismetSystemLibrary.LineTraceSingleForObjects` (`Actor.K2_GetActorLocation` (`self.GetOwner`)) _array_element_2 (`|MakeArray` "ObjectTypeQuery1" (`|GetArrayItem` (`self.ExplosionTarget`))) false (`local.IgnoreList`) "ForDuration" true (struct :`R` 1.0 :`A` 1.0) (struct :`G` 1.0 :`A` 1.0) 2.0))
            (if (== (`.HitActor` (`GameplayStatics.BreakHitResult` _outhit)) _array_element)
              (`KismetArrayLibrary.Array_Add` (`local.ReturnActor`) _array_element)
              (if (`self.IsOnlyGetResult`)
                (break)
                (else
                  (bind _asi_damage_able (cast `/Game/WorkSpace/Programing/SDH/Components/InterfaceInclude/Actor/I_DamageAble` _array_element))
                  (if (`self.IsHealing`)
                    (`/Game/WorkSpace/Programing/SDH/Components/InterfaceInclude/Actor/I_DamageAble.GiveHeal` _asi_damage_able (`self.Damage/Heal Amount`))
                    (break)
                    (else
                      (`/Game/WorkSpace/Programing/SDH/Components/InterfaceInclude/Actor/I_DamageAble.GiveDamage` _asi_damage_able (`self.Damage/Heal Amount`) (`self.OffenseLevel`) (`Actor.K2_GetActorLocation` (`self.GetOwner`)) (`self.IsFromPlayer`) false)
                      (break)))))))))
      (return (`local.ReturnActor`)))))

(fn `GetBoxCorners`
  (params (Origin :type "Vector Structure") (BoxExtent :type "Vector Structure"))
  (returns (Corners :type "Array of Vector Structure"))
  (bind (_boxextent_x _boxextent_y _boxextent_z) (`KismetMathLibrary.BreakVector` (`local.BoxExtent`)))
  (bind (_boxextent_x_2 _boxextent_y_2 _boxextent_z_2) (`KismetMathLibrary.BreakVector` (`local.BoxExtent`)))
  (bind (_boxextent_x_3 _boxextent_y_3 _boxextent_z_3) (`KismetMathLibrary.BreakVector` (`local.BoxExtent`)))
  (bind (_boxextent_x_4 _boxextent_y_4 _boxextent_z_4) (`KismetMathLibrary.BreakVector` (`local.BoxExtent`)))
  (bind (_boxextent_x_5 _boxextent_y_5 _boxextent_z_5) (`KismetMathLibrary.BreakVector` (`local.BoxExtent`)))
  (bind (_boxextent_x_6 _boxextent_y_6 _boxextent_z_6) (`KismetMathLibrary.BreakVector` (`local.BoxExtent`)))
  (bind (_boxextent_x_7 _boxextent_y_7 _boxextent_z_7) (`KismetMathLibrary.BreakVector` (`local.BoxExtent`)))
  (bind (_boxextent_x_8 _boxextent_y_8 _boxextent_z_8) (`KismetMathLibrary.BreakVector` (`local.BoxExtent`)))
  (bind _returnvalue (* (`self.ExplosionRayMoveAmount`) -1.0))
  (return (`|MakeArray` (`local.Origin`) (+ (`local.Origin`) (`KismetMathLibrary.MakeVector` _boxextent_x_2 0.0 _boxextent_z_2)) (+ (`local.Origin`) (`KismetMathLibrary.MakeVector` (* _boxextent_x_3 _returnvalue) 0.0 _boxextent_z_3)) (+ (`local.Origin`) (`KismetMathLibrary.MakeVector` 0.0 _boxextent_y_4 _boxextent_z_4)) (+ (`local.Origin`) (`KismetMathLibrary.MakeVector` 0.0 (* _boxextent_x_5 _returnvalue) _boxextent_z_5)) (+ (`local.Origin`) (`KismetMathLibrary.MakeVector` _boxextent_x_8 0.0 (* _boxextent_z_8 _returnvalue))) (+ (`local.Origin`) (`KismetMathLibrary.MakeVector` (* _boxextent_x _returnvalue) 0.0 (* _boxextent_z _returnvalue))) (+ (`local.Origin`) (`KismetMathLibrary.MakeVector` 0.0 _boxextent_y_6 (* _boxextent_z_6 _returnvalue))) (+ (`local.Origin`) (`KismetMathLibrary.MakeVector` 0.0 (* _boxextent_x_7 _returnvalue) (* _boxextent_z_7 _returnvalue))))))