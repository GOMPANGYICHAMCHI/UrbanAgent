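; Actor component that gates an emergency avoid (dodge) action behind a cooldown.
; EmergencyAvoid returns false while unavailable; otherwise it clears the availability flag, fires EmergencyAvoidActive and returns true.
; That event starts a one-shot timer using EmergencyCoolDown, whose reset event makes the avoid available again.
; The component holds only availability and timing, with no movement or animation logic.
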(event `EmergencyAvoidActive`
  ;[0.2083 0.2083 0.2083] 긴급회피 발동시 이벤트
  (`KismetSystemLibrary.K2_SetTimerDelegate` (delegate `EmergencyAvoidReset`) (`self.EmergencyCoolDown`)))

(event `EmergencyAvoidReset`
  ;[0.2083 0.2083 0.2083] 긴급회피 발동시 이벤트
  (set `self.EnergencyAvoidAvailable` true))

(fn `EmergencyAvoid`
  (returns (IsActive :type Boolean))
  (if (`self.EnergencyAvoidAvailable`)
    (set `self.EnergencyAvoidAvailable` false)
    (`self.EmergencyAvoidActive`)
    (return true)
    (else
      (return false))))