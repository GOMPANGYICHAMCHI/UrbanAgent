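; AC_Damageable is an actor component that holds health and applies damage and healing to it.
; Player damage subtracts a defense ratio, built from DefensePower and the other side's offense level, from the incoming amount.
; Monster damage instead scales the amount by a linear factor of the component's own OffenseLevel.
; Damage and healing clamp health between zero and maximum, and RatioHealth returns the current fraction.
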(fn `GiveDamage(Monster)`
  (params (DamageAmount :type "Float (double-precision)"))
  (locals (A :type "Float (double-precision)" :default 1.0) (B :type "Float (double-precision)" :default 20.0))
  (set `self.HealthPoint` (`KismetMathLibrary.FClamp` (- (`self.HealthPoint`) (* (- 1.0 (/ (- (`self.OffenseLevel`) (`local.A`)) (`local.B`))) (`local.DamageAmount`))) 0.0 (`self.MaxHealthPoint`))))

(fn `GiveDamage(Player)`
  (params (DamageAmount :type "Float (double-precision)") (OtherOffenseLevel :type "Float (double-precision)"))
  (locals (K :type "Float (double-precision)" :default 500.0) (N :type "Float (double-precision)" :default 100.0))
  (set `self.HealthPoint` (`KismetMathLibrary.FClamp` (- (`self.HealthPoint`) (- DamageAmount (/ (`self.DefensePower`) (+ (+ (* (`local.OtherOffenseLevel`) (`local.K`)) (`local.N`)) (`self.DefensePower`))))) 0.0 (`self.MaxHealthPoint`))))

(fn `GiveHeal`
  (params (HealAmount :type "Float (double-precision)"))
  (set `self.HealthPoint` (`KismetMathLibrary.FClamp` (+ (`self.HealthPoint`) HealAmount) 0.0 (`self.MaxHealthPoint`))))

(fn `RatioHealth`
  (returns (RatioHealth :type "Float (double-precision)"))
  (return (/ (`self.HealthPoint`) (`self.MaxHealthPoint`))))