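; BP_PlayerNewClose is a child player character for close combat, carrying a bat as a child actor.
; BeginPlay binds skill, ultimate, reset and dodge delegates and caches the bat and ring meshes.
; Skill and ultimate events set the player state and play their montages, restoring the state when completed or interrupted; reset delegates also restore it.
; Perfect dodge applies an overlay material to bat and ring until dash end clears it.
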(event `self.ReceiveBeginPlay`
  (bind _asbp_new_close_bat (cast `/Game/WorkSpace/Programing/SDH/Actors/Players/BP_NewCloseBat` (`ChildActorComponent.ChildActor` (`self.BP_NewCloseBat`)) :!pure true))
  (`parent.ReceiveBeginPlay`)
  (add `self.SkillUseStart` (`|CreateDelegate` :!event `UseSkillActual`))
  (add `self.UltimateSkillUseStart` (`|CreateDelegate` :!event `UseUltimateSkillActual`))
  (add `self.SC_ResetSkill` (delegate `ResetSkill`))
  (add `self.SC_ResetUltimateSkill` (delegate `ResetSkill`))
  (set `self.c_Batring` (`/Game/WorkSpace/Programing/SDH/Actors/Players/BP_NewCloseBat.Ring` _asbp_new_close_bat))
  (set `self.c_Bat` (`/Game/WorkSpace/Programing/SDH/Actors/Players/BP_NewCloseBat.Bat` _asbp_new_close_bat))
  (add `self.PerfectDodge` (delegate `PefectDodge`))
  (add `self.DashEnd` (delegate `DashEnd_actual`)))

(event `ResetSkill`
  (set `self.CurrentPlayerState` "NewEnumerator4"))

(event `PefectDodge`
  (`MeshComponent.SetOverlayMaterial` (`self.c_Bat`) "/Game/WorkSpace/Programing/SDH/Materials/MT_PlayerPerfectDodge.MT_PlayerPerfectDodge")
  (`MeshComponent.SetOverlayMaterial` (`self.c_Batring`) "/Game/WorkSpace/Programing/SDH/Materials/MT_PlayerPerfectDodge.MT_PlayerPerfectDodge"))

(event `DashEnd_actual`
  (`MeshComponent.SetOverlayMaterial` (`self.c_Bat`) null)
  (`MeshComponent.SetOverlayMaterial` (`self.c_Batring`) null))

(event `UltimateSkillReset`)

(event `self.ReceiveTick`
  (params (DeltaSeconds :type "Float (single-precision)"))
  (`parent.ReceiveTick` DeltaSeconds))

(event `UseSkillActual`
  (set `self.CurrentPlayerState` "NewEnumerator10")
  (`self.StopAnimMontage` (`self.CurrentAnimMontage`))
  (set `self.CurrentAnimMontage` (`self.SkillAnimMontage`))
  (`|PlayMontage` (`self.Mesh`) (`self.CurrentAnimMontage`)
    (:`OnCompleted`
      _)
    (:`OnInterrupted`
      _))
  (set `self.CurrentPlayerState` "NewEnumerator4"))

(event `UseUltimateSkillActual`
  (set `self.CurrentPlayerState` "NewEnumerator11")
  (`self.StopAnimMontage` (`self.CurrentAnimMontage`))
  (set `self.CurrentAnimMontage` (`self.UltimateSkillAnimMontage`))
  (`|PlayMontage` (`self.Mesh`) (`self.CurrentAnimMontage`)
    (:`OnCompleted`
      _)
    (:`OnInterrupted`
      _))
  (set `self.CurrentPlayerState` "NewEnumerator4"))

(fn `UserConstructionScript`
  (`parent.UserConstructionScript`))