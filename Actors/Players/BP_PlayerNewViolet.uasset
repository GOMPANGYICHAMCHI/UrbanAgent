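; Player character Blueprint for Violet that extends a parent player class with skill, ultimate, dodge and swap reactions.
; BeginPlay binds handlers to the skill, reset, perfect dodge, dash end and player swap events.
; Skill and ultimate handlers set the player state and play their montage, restoring a shared state on completion or interruption.
; Perfect dodge puts an overlay material on hair and swords until dash end, and swapping makes the mesh visible.
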(event `SetVisib`
  (`SceneComponent.SetVisibility` (`self.Mesh`) true false))

(event `self.ReceiveBeginPlay`
  (`parent.ReceiveBeginPlay`)
  (add `self.SkillUseStart` (`|CreateDelegate` :!event `UseSkillActual`))
  (add `self.UltimateSkillUseStart` (`|CreateDelegate` :!event `UseUltimateSkillActual`))
  (add `self.SC_ResetSkill` (delegate `ResetSkill`))
  (add `self.SC_ResetUltimateSkill` (delegate `ResetSkill`))
  (add `self.PerfectDodge` (delegate `PefectDodge`))
  (add `self.DashEnd` (delegate `DashEnd_actual`))
  (add `self.PlayerSwaped` (delegate `SetVisib`)))

(event `ResetSkill`
  (set `self.CurrentPlayerState` "NewEnumerator4"))

(event `UltimateSkillReset`)

(event `PefectDodge`
  (`MeshComponent.SetOverlayMaterial` (`self.Hair`) "/Game/WorkSpace/Programing/SDH/Materials/MT_PlayerPerfectDodge.MT_PlayerPerfectDodge")
  (`MeshComponent.SetOverlayMaterial` (`self.Sword`) "/Game/WorkSpace/Programing/SDH/Materials/MT_PlayerPerfectDodge.MT_PlayerPerfectDodge")
  (`MeshComponent.SetOverlayMaterial` (`self.Sword1`) "/Game/WorkSpace/Programing/SDH/Materials/MT_PlayerPerfectDodge.MT_PlayerPerfectDodge"))

(event `DashEnd_actual`
  (`MeshComponent.SetOverlayMaterial` (`self.Hair`) null)
  (`MeshComponent.SetOverlayMaterial` (`self.Sword`) null)
  (`MeshComponent.SetOverlayMaterial` (`self.Sword1`) null))

(event `self.ReceiveTick`
  (params (DeltaSeconds :type "Float (single-precision)"))
  (`parent.ReceiveTick` DeltaSeconds))

(event `UseSkillActual`
  (set `self.CurrentPlayerState` "NewEnumerator10")
  (`self.StopAnimMontage` (`self.CurrentAnimMontage`))
  (set `self.CurrentAnimMontage` (`self.SkillAnimMontage`))
  (`|PlayMontage` (`self.Mesh`) (`self.CurrentAnimMontage`)
    (:`OnCompleted`
      _)
    (:`OnInterrupted`
      _))
  (set `self.CurrentPlayerState` "NewEnumerator4"))

(event `UseUltimateSkillActual`
  (set `self.CurrentPlayerState` "NewEnumerator11")
  (`self.StopAnimMontage` (`self.CurrentAnimMontage`))
  (set `self.CurrentAnimMontage` (`self.UltimateSkillAnimMontage`))
  (`|PlayMontage` (`self.Mesh`) (`self.CurrentAnimMontage`)
    (:`OnCompleted`
      _)
    (:`OnInterrupted`
      _))
  (set `self.CurrentPlayerState` "NewEnumerator4"))

(fn `UserConstructionScript`
  (`parent.UserConstructionScript`))