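; BP_LockOnCrossHair is an actor that shows a lock-on crosshair through its Widget component over a targeted actor.
; SetTarget stores the target and, if valid, saves a position offset and shows the widget.
; While the widget is visible, Tick moves the crosshair to the target's location plus that offset.
; OnOff and IsOn set and report visibility, and an optional DestroySelf flag removes the actor one second after BeginPlay.
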(event `self.ReceiveBeginPlay`
  (if (`self.DestroySelf`)
    (`KismetSystemLibrary.Delay` 1.0)
    (`self.K2_DestroyActor`)))

(event `self.ReceiveTick`
  (params (DeltaSeconds :type "Float (single-precision)"))
  (if (`SceneComponent.bVisible` (`self.Widget`))
    (if (`KismetSystemLibrary.IsValid` (`self.CurrentTarget`))
      (`self.K2_SetActorLocation` (+ (`self.K2_GetActorLocation` (`self.CurrentTarget`)) (`self.Adjustment`))))))

(fn `IsOn`
  (returns (IsOn :type Boolean))
  (return (`SceneComponent.bVisible` (`self.Widget`))))

(fn `OnOff`
  (params (IsOn :type Boolean))
  (`SceneComponent.SetVisibility` (`self.Widget`) IsOn false))

(fn `SetTarget`
  (params (NewTarget :type "Actor Object Reference") (Adjustment :type "Vector Structure"))
  (set `self.CurrentTarget` NewTarget)
  (`/Engine/EditorBlueprintResources/StandardMacros.IsValid` (`self.CurrentTarget`)
    (:`Is Valid`
      (set `self.Adjustment` Adjustment)
      (`SceneComponent.SetVisibility` (`self.Widget`) true false))))

(fn `UserConstructionScript`)