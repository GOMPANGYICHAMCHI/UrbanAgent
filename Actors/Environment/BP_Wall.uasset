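; BP_Wall is an environment barrier made of two poles, arrow panels, a black background and a collision box.
; The construction script uses Length to space the poles apart and stretch the box, background and three panels to match, giving a resizable wall.
; SetActive stores the state in CurrentActive and toggles visibility of the poles, panels and background, along with collision on the poles and box.
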(fn `SetActive`
  (params (IsActive :type Boolean))
  (bind _box (`self.Box`))
  (set `self.CurrentActive` IsActive)
  (`SceneComponent.SetVisibility` (`self.Arrowpanel_middle`) (`local.IsActive`) false)
  (`SceneComponent.SetVisibility` (`self.Arrowpanel_down`) (`local.IsActive`) false)
  (`SceneComponent.SetVisibility` (`self.Arrowpanel_up`) (`local.IsActive`) false)
  (`SceneComponent.SetVisibility` (`self.BlackBackground`) (`local.IsActive`) false)
  (`SceneComponent.SetVisibility` (`self.Pole_Left`) (`local.IsActive`) false)
  (`SceneComponent.SetVisibility` (`self.Pole_Right`) (`local.IsActive`) false)
  (if (`local.IsActive`)
    (`PrimitiveComponent.SetCollisionEnabled` (`self.Pole_Left`) "QueryAndPhysics")
    (`PrimitiveComponent.SetCollisionEnabled` (`self.Pole_Right`) "QueryAndPhysics")
    (`PrimitiveComponent.SetCollisionEnabled` _box "QueryAndPhysics")
    (else
      (`PrimitiveComponent.SetCollisionEnabled` (`self.Pole_Left`) "NoCollision")
      (`PrimitiveComponent.SetCollisionEnabled` (`self.Pole_Right`) "NoCollision")
      (`PrimitiveComponent.SetCollisionEnabled` _box "NoCollision"))))

(fn `UserConstructionScript`
  (bind _returnvalue (+ (* (`self.Length`) 3.0) 3.0))
  (`SceneComponent.K2_SetRelativeLocation` (`self.Pole_Right`) (`KismetMathLibrary.MakeVector` (`KismetMathLibrary.Conv_IntToDouble` (+ (* (`self.Length`) 150) 165)) 0.0 -120.0) false false)
  (`SceneComponent.K2_SetRelativeLocation` (`self.Pole_Left`) (`KismetMathLibrary.MakeVector` (`KismetMathLibrary.Conv_IntToDouble` (+ (* (`self.Length`) -150) -165)) 0.0 -120.0) false false)
  (`SceneComponent.SetRelativeScale3D` (`self.Box`) (`KismetMathLibrary.MakeVector` (`KismetMathLibrary.Conv_IntToDouble` (+ (* (`self.Length`) 5) 5)) 1.0 16.0))
  (`SceneComponent.SetRelativeScale3D` (`self.BlackBackground`) (`KismetMathLibrary.MakeVector` (`KismetMathLibrary.Conv_IntToDouble` (+ (* (`self.Length`) 3) 3)) 2.2 1.0))
  (`SceneComponent.SetRelativeScale3D` (`self.Arrowpanel_up`) (`KismetMathLibrary.MakeVector` _returnvalue 0.6 1.0))
  (`SceneComponent.SetRelativeScale3D` (`self.Arrowpanel_down`) (`KismetMathLibrary.MakeVector` _returnvalue 0.6 1.0))
  (`SceneComponent.SetRelativeScale3D` (`self.Arrowpanel_middle`) (`KismetMathLibrary.MakeVector` (+ (* (`self.Length`) 3.0) 3.0) 0.8 1.0)))