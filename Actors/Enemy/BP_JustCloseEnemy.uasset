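; Close-range enemy Blueprint that extends its parent enemy with visuals for two robot arm meshes.
; Parent event overrides mirror execution overlays and lock-on custom depth onto both arms, clearing the overlay on death.
; BeginPlay binds death and attacked callbacks, which hide the billboard and fire a hit spark.
; Sword collision, debug state text and dissolve logic are disconnected, and GetDesireDirection returns a zero vector.
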(event `self.EnemyDeath`
  (`parent.EnemyDeath`)
  (`MeshComponent.SetOverlayMaterial` (`self.RobotArm_R`) null)
  (`MeshComponent.SetOverlayMaterial` (`self.RobotArm_L`) null))

(event `self.ReceiveTick`
  (params (DeltaSeconds :type "Float (single-precision)"))
  (`parent.ReceiveTick` DeltaSeconds))

(event `self.SetExcution`
  (params (TargetAnimation :type "AnimMontage Object Reference"))
  (`parent.SetExcution` TargetAnimation)
  (`MeshComponent.SetOverlayMaterial` (`self.RobotArm_R`) null)
  (`MeshComponent.SetOverlayMaterial` (`self.RobotArm_L`) null))

(event `PlayerHitted`
  (set `self.IsPlayerHit` true))

(event `self.CanExcution_Actual`
  (params (IsTrue :type Boolean))
  (`parent.CanExcution_Actual` IsTrue)
  (`MeshComponent.SetOverlayMaterial` (`self.RobotArm_R`) "/Game/WorkSpace/Programing/SDH/Materials/MT_EnemyExcutionOverlay.MT_EnemyExcutionOverlay")
  (`MeshComponent.SetOverlayMaterial` (`self.RobotArm_L`) "/Game/WorkSpace/Programing/SDH/Materials/MT_EnemyExcutionOverlay.MT_EnemyExcutionOverlay"))

(event `DeadActual_event`
  ;[1 1 1] 사망 이벤트
  (`SceneComponent.SetVisibility` (`self.Billboard`) false false))

(event `self.ReceiveBeginPlay`
  ;[1 1 1] 시작시 이벤트 설정
  (`parent.ReceiveBeginPlay`)
  (add `self.DeadActual` (`|CreateDelegate` :!event `DeadActual_event`))
  (add `self.Attacked` (delegate `HitParticle`)))

(event `HitParticle`
  ;[1 1 1] 시작시 이벤트 설정
  (`ActorComponent.SetActive` (`self.P_HitSpark`) true true))

(event `/Game/WorkSpace/Programing/SDH/Interface/Actor/I_CloseAttacker.SwordOnOff`
  (params (IsOn :type Boolean) (Size :type "Float (double-precision)") (DamagePercent :type "Float (double-precision)") (Duration :type "Float (double-precision)") (InputAttackData :type "Array of /Game/WorkSpace/Programing/SDH/EnumStruct/S_AttackData Structure (by ref)") (InputKnockbackData :type "Array of /Game/WorkSpace/Programing/SDH/EnumStruct/S_KnockBackData Structure (by ref)") (HitCameraShake :type "CameraShakeBase Class Reference") (InputBulletTimeData :type "/Game/WorkSpace/Programing/SDH/EnumStruct/S_BulletTimeData Structure"))
  ;[0.1615 0.1615 0.1615] 공격 콜리전 ON/OFF
)

(event `/Game/WorkSpace/Programing/SDH/Components/InterfaceInclude/Actor/I_DamageAble.GetLockOn`
  (params (IsOn :type Boolean))
  (`parent.GetLockOn` IsOn)
  (`PrimitiveComponent.SetRenderCustomDepth` (`self.RobotArm_L`) IsOn)
  (`PrimitiveComponent.SetRenderCustomDepth` (`self.RobotArm_R`) IsOn))

(fn `GetDesireDirection`
  (returns (DirectionVelocity :type "Vector Structure"))
  (return (0.0 0.0 0.0)))

(fn `UserConstructionScript`)