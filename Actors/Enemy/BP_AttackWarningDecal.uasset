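; BP_AttackWarningDecal is an enemy attack warning indicator whose Fill component grows to show progress over a given duration.
; SetDecalOn stores the duration, resets the fill, and plays the SetOn timeline at that length.
; The timeline serves as a ticker, accumulating world delta seconds to scale Fill along Y by elapsed over total time.
; On finish, the fill amount and Y scale reset to zero.
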(event `SetDecalOn`
  (params (Time :type "Float (double-precision)"))
  (set `self.Time` Time)
  (set `self.FillAmount` 0.0)
  (`SceneComponent.SetRelativeScale3D` (`self.Fill`) (0.0 1.0 0.02))
  (`TimelineComponent.SetTimelineLength` (`self.SetOn`) (`self.Time`))
  (`Timeline|SetOn` :!via `PlayFromStart`
    (:`Update`
      (set `self.FillAmount` (+ (`self.FillAmount`) (`GameplayStatics.GetWorldDeltaSeconds`)))
      (`SceneComponent.SetRelativeScale3D` (`self.Fill`) (`KismetMathLibrary.MakeVector` 1.0 (/ (`self.FillAmount`) (`self.Time`)) 0.02)))
    (:`Finished`
      (set `self.FillAmount` 0.0)
      (`SceneComponent.SetRelativeScale3D` (`self.Fill`) (1.0 0.0 0.02)))))

(fn `UserConstructionScript`)